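; BP_FloatText is a proximity-triggered floating text prop with an accompanying point light.
; The construction script applies the text, light intensity and light color from Blueprint variables.
; BeginPlay hides only the text; a component tagged "P" entering Box15 makes both text and light visible.
; The reveal is one-way, as no end-overlap logic hides them again.
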(event OnComponentBeginOverlap(box15)
  (params (OverlappedComponent :type Primitive%20Component%20Object%20Reference) (OtherActor :type Actor%20Object%20Reference) (OtherComp :type Primitive%20Component%20Object%20Reference) (OtherBodyIndex :type Integer) (bFromSweep :type Boolean) (SweepResult :type Hit%20Result%20Structure%20%28by%20ref%29))
  (if (Components|ComponentHasTag OtherComp "P")
    (Rendering|SetVisibility (Variables|Default|GetPointLight) true false)))

(event EventBeginPlay
  (Rendering|SetVisibility (Variables|Default|GetTextRenderMy) false false))

(event Collision|EventActorBeginOverlap
  (params (OtherActor :type Actor%20Object%20Reference)))

(event EventTick
  (params (DeltaSeconds :type Float%20%28single-precision%29)))

(fn ConstructionScript
  (Rendering|Components|TextRender|SetText (Variables|Default|GetTextRenderMy) (Variables|Text|GetMy%20Text%20Value))
  (Rendering|Components|Light|SetIntensity (Variables|Default|GetPointLight) (Variables|Light|GetNew%20Intensity))
  (Rendering|Components|Light|SetLightColor (Variables|Default|GetPointLight) (Variables|Light|GetNew%20Light%20Color) true))