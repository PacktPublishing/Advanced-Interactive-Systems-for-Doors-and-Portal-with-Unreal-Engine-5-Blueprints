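; BP_Button is an interactable puzzle button that toggles on and off with E and reports its state to a PuzzleManager.
; Box overlap with a "P"-tagged component enables input and shows a Turn On/Turn Off prompt through the third-person game mode.
; A Timeline played forward or reversed slides the mesh, blocking presses mid-animation.
; When it finishes, the button swaps material, refreshes the prompt and notifies the manager.
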(event OnComponentBeginOverlap(Box)
  (params (OverlappedComponent :type Primitive%20Component%20Object%20Reference) (OtherActor :type Actor%20Object%20Reference) (OtherComp :type Primitive%20Component%20Object%20Reference) (OtherBodyIndex :type Integer) (bFromSweep :type Boolean) (SweepResult :type Hit%20Result%20Structure%20%28by%20ref%29))
  (if (Components|ComponentHasTag OtherComp "P")
    (Input|EnableInput (Game|GetPlayerController 0))
    (CallFunction|UpdateWidgetText)
    (Default|AddDoorWidget (Variables|Default|GetAs%20BP%20Third%20Person%20Game%20Mode) (Variables|Default|GetBox))))

(event OnComponentEndOverlap(Box)
  (params (OverlappedComponent :type Primitive%20Component%20Object%20Reference) (OtherActor :type Actor%20Object%20Reference) (OtherComp :type Primitive%20Component%20Object%20Reference) (OtherBodyIndex :type Integer))
  (if (Components|ComponentHasTag OtherComp "P")
    (Input|DisableInput (Game|GetPlayerController 0))
    (CallFunction|UpdateWidgetText)
    (Default|RemoveDoorWidget (Variables|Default|GetAs%20BP%20Third%20Person%20Game%20Mode))))

(event EventBeginPlay
  (bind _asbp_third_person_game_mode (Utilities|Casting|CastToBP_ThirdPersonGameMode (Game|GetGameMode)))
  (Variables|Default|SetAs%20BP%20Third%20Person%20Game%20Mode _asbp_third_person_game_mode))

(event Collision|EventActorBeginOverlap
  (params (OtherActor :type Actor%20Object%20Reference)))

(event EventTick
  (params (DeltaSeconds :type Float%20%28single-precision%29)))

(event Input|KeyboardEvents|E
  (params (Key :type Key%20Structure :default "None"))
  (bind _self self)
  (bind _puzzle_manager (Variables|Default|GetPuzzle%20Manager))
  (:Pressed
    (if (not (Audio|Components|Audio|IsPlaying (Variables|Default|GetTimeline)))
      (Audio|PlaySound2D "/Game/Sounds/Button_Cue.Button_Cue" 1.0 1.0 0.0 0 0)
      (if (Variables|Default|GetIs%20On)
        (Variables|Default|SetIs%20On false)
        (bind _newtrack_0 (Timeline|Timeline Reverse)
          (:Update
            (Transformation|SetRelativeLocation (Variables|Default|GetStaticMesh) (Math|Vector|MakeVector 0.0 (Math|Float|Lerp 0.0 -0.3 _newtrack_0) 0.0) false false))
          (:Finished
            (Rendering|Material|SetMaterial (Variables|Default|GetStaticMesh) 0 (select (Variables|Default|GetIs%20On) "/Game/Assets/Textures/PropsOn.PropsOn" "/Game/Assets/Textures/Props.Props"))
            (CallFunction|UpdateWidgetText)
            (if (Variables|Default|GetIs%20On)
              (Default|Buttonon _puzzle_manager _self)
              (else
                (Default|ButtonOff _puzzle_manager _self)))))
        (else
          (Variables|Default|SetIs%20On true)
          (Timeline|Timeline Play))))))

(fn ConstructionScript)

(fn UpdateWidgetText
  (bind _as_bp_third_person_game_mode (Variables|Default|GetAs%20BP%20Third%20Person%20Game%20Mode))
  (if (Variables|Default|GetIs%20On)
    (Default|UpdateWidgetText _as_bp_third_person_game_mode "Turn Off")
    (else
      (Default|UpdateWidgetText _as_bp_third_person_game_mode "Turn On"))))