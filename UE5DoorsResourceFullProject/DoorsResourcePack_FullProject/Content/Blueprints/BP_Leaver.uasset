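; One-shot lever switch that unlocks its assigned door when the player uses it.
; Box overlap with a "P"-tagged component toggles actor input and the "Use" prompt handled through BP_ThirdPersonGameMode.
; Pressing E sets IsSolved, plays a pitch-randomized sound and rotates the mesh along a timeline.
; When the timeline finishes, it swaps to the PropsOn material and sends UnlockDoorMessage to DoorActor via BI_Doors.
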(event OnComponentBeginOverlap(Box)
  (params (OverlappedComponent :type Primitive%20Component%20Object%20Reference) (OtherActor :type Actor%20Object%20Reference) (OtherComp :type Primitive%20Component%20Object%20Reference) (OtherBodyIndex :type Integer) (bFromSweep :type Boolean) (SweepResult :type Hit%20Result%20Structure%20%28by%20ref%29))
  (if (Components|ComponentHasTag OtherComp "P")
    (Input|EnableInput (Game|GetPlayerController 0))
    (CallFunction|UpdateWidgetText)
    (Default|AddDoorWidget (Variables|Default|GetAs%20BP%20Third%20Person%20Game%20Mode) (Variables|Default|GetBox))))

(event OnComponentEndOverlap(Box)
  (params (OverlappedComponent :type Primitive%20Component%20Object%20Reference) (OtherActor :type Actor%20Object%20Reference) (OtherComp :type Primitive%20Component%20Object%20Reference) (OtherBodyIndex :type Integer))
  (if (Components|ComponentHasTag OtherComp "P")
    (Input|DisableInput (Game|GetPlayerController 0))
    (CallFunction|UpdateWidgetText)
    (Default|RemoveDoorWidget (Variables|Default|GetAs%20BP%20Third%20Person%20Game%20Mode))))

(event EventBeginPlay
  (bind _asbp_third_person_game_mode (Utilities|Casting|CastToBP_ThirdPersonGameMode (Game|GetGameMode)))
  (Variables|Default|SetAs%20BP%20Third%20Person%20Game%20Mode _asbp_third_person_game_mode)
  (Variables|Default|SetRelative%20Rotation (Variables|/Script/Engine.SceneComponent|GetRelativeRotation (Variables|Default|GetStaticMesh1))))

(event Collision|EventActorBeginOverlap
  (params (OtherActor :type Actor%20Object%20Reference)))

(event EventTick
  (params (DeltaSeconds :type Float%20%28single-precision%29)))

(event Input|KeyboardEvents|E
  (params (Key :type Key%20Structure :default "None"))
  (bind _relative_rotation (Variables|Default|GetRelative%20Rotation))
  (bind _door_actor (Variables|Default|GetDoor%20Actor))
  (bind (_roll _pitch _yaw) (Math|Rotator|BreakRotator _relative_rotation))
  (:Pressed
    (if (not (Variables|Default|GetIsSolved))
      (Variables|Default|SetIsSolved true)
      (CallFunction|UpdateWidgetText)
      (Audio|PlaySound2D "/Game/Sounds/Leaver_Cue.Leaver_Cue" 1.0 (Math|Random|RandomFloatinRange 0.8 1.0) 0.0 0 0)
      (bind _newtrack_0 (Timeline|Timeline Play)
        (:Update
          (Transformation|SetRelativeRotation (Variables|Default|GetStaticMesh1) (Math|Rotator|Lerp(Rotator) _relative_rotation (Math|Rotator|MakeRotator _roll 1.8e+02 _yaw) _newtrack_0 true) false false))
        (:Finished
          (Rendering|Material|SetMaterial (Variables|Default|GetStaticMesh1) 0 "/Game/Assets/Textures/PropsOn.PropsOn")
          (Utilities|IsValid _door_actor
            (:Is%20Valid
              (if (Utilities|DoesObjectImplementInterface _door_actor "/Game/Blueprints/BI_Doors.BI_Doors_C")
                (Class|BIDoors|UnlockDoor(Message) _door_actor)
                (else
                  (Development|PrintString "Error Switch Actor Dosnt Implement Interface"))))
            (:Is%20Not%20Valid
              (Development|PrintString "Error Switch dosnt have an actor"))))))))

(fn ConstructionScript)

(fn UpdateWidgetText
  (bind _as_bp_third_person_game_mode (Variables|Default|GetAs%20BP%20Third%20Person%20Game%20Mode))
  (if (Variables|Default|GetIsSolved)
    (Default|RemoveDoorWidget _as_bp_third_person_game_mode)
    (else
      (Default|UpdateWidgetText _as_bp_third_person_game_mode "Use"))))

(fn Solved
  (return (Variables|Default|GetIsSolved)))