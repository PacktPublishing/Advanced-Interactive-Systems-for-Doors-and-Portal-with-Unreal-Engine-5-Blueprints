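; Key-locked sci-fi door with two vertically sliding panels, operated with E while the tagged player is inside its trigger box.
; Unlocking consumes the required inventory item, while failure plays a denial sound and flashes the material red via a DoN/FlipFlop delay loop.
; Once unlocked, a reversible timeline slides the panels and updates DoorState, which sets the prompt text shown through the game mode's door widget.
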(event OnComponentBeginOverlap(Box)
  (params (OverlappedComponent :type Primitive%20Component%20Object%20Reference) (OtherActor :type Actor%20Object%20Reference) (OtherComp :type Primitive%20Component%20Object%20Reference) (OtherBodyIndex :type Integer) (bFromSweep :type Boolean) (SweepResult :type Hit%20Result%20Structure%20%28by%20ref%29))
  (if (Components|ComponentHasTag OtherComp "P")
    (Input|EnableInput (Game|GetPlayerController 0))
    (CallFunction|UpdateWidgetText)
    (Default|AddDoorWidget (Variables|Default|GetAs%20BP%20Third%20Person%20Game%20Mode) (Variables|Default|GetBox))))

(event OnComponentEndOverlap(Box)
  (params (OverlappedComponent :type Primitive%20Component%20Object%20Reference) (OtherActor :type Actor%20Object%20Reference) (OtherComp :type Primitive%20Component%20Object%20Reference) (OtherBodyIndex :type Integer))
  (if (Components|ComponentHasTag OtherComp "P")
    (Input|DisableInput (Game|GetPlayerController 0))
    (CallFunction|UpdateWidgetText)
    (Default|RemoveDoorWidget (Variables|Default|GetAs%20BP%20Third%20Person%20Game%20Mode))))

(event Custom|Door%20Animation
  (switch Utilities|FlowControl|Switch|SwitchonE_DoorState (Variables|Default|GetDoor%20State)
    (:NewEnumerator0
      (if (== (Components|Timeline|GetPlaybackPosition (Variables|Default|GetAnimation%20Timeline)) 0.0)
        (bind (_direction _door_rotation_alpha) (Timeline|Animation%20Timeline Reverse)
          (:Update
            (Transformation|SetRelativeLocation (Variables|Default|GetPropPackUE_Door1) (Math|Vector|MakeVector 0.0 5e+01 (Math|Float|Lerp 125.0 2.2e+02 _door_rotation_alpha)) false false)
            (Transformation|SetRelativeLocation (Variables|Default|GetPropPackUE_Door2) (Math|Vector|MakeVector 0.0 5e+01 (Math|Float|Lerp 115.0 -5.0 _door_rotation_alpha)) false false)
            (Utilities|FlowControl|DoOnce false :!label _label
              (:Completed
                (switch Utilities|FlowControl|Switch|SwitchonETimelineDirection _direction
                  (:Forward
                    (Variables|Default|SetDoor%20State "NewEnumerator2"))
                  (:Backward
                    (Variables|Default|SetDoor%20State "NewEnumerator3")))
                (Default|RemoveDoorWidget (Variables|Default|GetAs%20BP%20Third%20Person%20Game%20Mode)))))
          (:Finished
            (Utilities|FlowControl|Sequence
              (:then_0
                (switch Utilities|FlowControl|Switch|SwitchonETimelineDirection _direction
                  (:Forward
                    (Variables|Default|SetDoor%20State "NewEnumerator0"))
                  (:Backward
                    (Variables|Default|SetDoor%20State "NewEnumerator1")))
                (Default|AddDoorWidget (Variables|Default|GetAs%20BP%20Third%20Person%20Game%20Mode) (Variables|Default|GetBox))
                (CallFunction|UpdateWidgetText))
              (:then_1
                (goto _label Reset)))))
        (else
          (Audio|PlaySound2D "/Game/Sounds/scifiDoor_Cue.scifiDoor_Cue" 1.0 0.8 0.0 0 0)
          (Timeline|Animation%20Timeline Reverse))))
    (:NewEnumerator1
      (Audio|PlaySound2D "/Game/Sounds/scifiDoor_Cue.scifiDoor_Cue" 1.0 1.0 0.0 0 0)
      (Timeline|Animation%20Timeline Play))))

(event Custom|Lock%20Mechanism
  (bind _key_found (CallFunction|CheckforKey))
  (if _key_found
    (Variables|Default|SetDoor%20State "NewEnumerator1")
    (CallFunction|UpdateWidgetText)
    (Rendering|Material|SetMaterial (Variables|Default|GetPropPackUE_Door1) 0 "/Game/Assets/Textures/DoorVerticalSOpen.DoorVerticalSOpen")
    (Audio|PlaySound2D "/Game/Sounds/Button_Cue.Button_Cue" 1.0 1.0 0.0 0 0)
    (else
      (CallFunction|ResetDoNRattle)
      (Audio|PlaySound2D "/Game/Sounds/582632__ironcross32__permission-denied_Cue.582632__ironcross32__permission-denied_Cue" 1.0 1.0 0.0 0 0)
      (CallFunction|Rattle))))

(event Custom|Rattle
  (Utilities|FlowControl|DoN 4
    (:Exit
      (Utilities|FlowControl|Delay 0.1)
      (bind _isa (Utilities|FlowControl|FlipFlop)
        (:A
          _)
        (:B
          _))
      (Rendering|Material|SetMaterial (Variables|Default|GetPropPackUE_Door1) 0 (select _isa "/Game/Assets/Textures/DoorVerticalRed.DoorVerticalRed" "/Game/Assets/Textures/DoorVerticalS.DoorVerticalS"))
      (CallFunction|Rattle))))

(event Custom|Reset%20Do%20N%20Rattle
  (Utilities|FlowControl|DoN 4) ; enters at Reset
)

(event EventBeginPlay
  (bind _asbp_third_person_game_mode (Utilities|Casting|CastToBP_ThirdPersonGameMode (Game|GetGameMode)))
  (Variables|Default|SetAs%20BP%20Third%20Person%20Game%20Mode _asbp_third_person_game_mode))

(event Collision|EventActorBeginOverlap
  (params (OtherActor :type Actor%20Object%20Reference)))

(event EventTick
  (params (DeltaSeconds :type Float%20%28single-precision%29)))

(event Input|KeyboardEvents|E
  (params (Key :type Key%20Structure :default "None"))
  (:Pressed
    (if (Utilities|Enum|Equal(Enum) (Variables|Default|GetDoor%20State) "NewEnumerator4")
      (CallFunction|LockMechanism)
      (else
        (CallFunction|DoorAnimation)))))

(fn ConstructionScript)

(fn UpdateWidgetText
  (switch Utilities|FlowControl|Switch|SwitchonE_DoorState (Variables|Default|GetDoor%20State)
    (:NewEnumerator0
      (Default|UpdateWidgetText (Variables|Default|GetAs%20BP%20Third%20Person%20Game%20Mode) "Close"))
    (:NewEnumerator1
      (Default|UpdateWidgetText (Variables|Default|GetAs%20BP%20Third%20Person%20Game%20Mode) "Open"))
    (:NewEnumerator2
      (Default|UpdateWidgetText (Variables|Default|GetAs%20BP%20Third%20Person%20Game%20Mode) :!label _label))
    (:NewEnumerator3
      (goto _label))
    (:NewEnumerator4
      (Default|UpdateWidgetText (Variables|Default|GetAs%20BP%20Third%20Person%20Game%20Mode) "Locked"))))

(fn CheckforKey
  (bind _returnvalue (Game|Player|GetPlayerPawn 0))
  (bind _required_item (Variables|Default|GetRequired%20Item))
  (bind _asbp_third_person_character (Utilities|Casting|CastToBP_ThirdPersonCharacter _returnvalue))
  (bind _inventory (Variables|/Game/ThirdPerson/Blueprints/BP_ThirdPersonCharacter.BP_ThirdPersonCharacter_C|GetInventory _asbp_third_person_character))
  (bind _returnvalue_2 (Utilities|Array|FindItem _inventory _required_item))
  (if (>= _returnvalue_2 0)
    (Utilities|Array|RemoveIndex (Variables|/Game/ThirdPerson/Blueprints/BP_ThirdPersonCharacter.BP_ThirdPersonCharacter_C|GetInventory (.AsBP%20Third%20Person%20Character (Utilities|Casting|CastToBP_ThirdPersonCharacter (Game|Player|GetPlayerPawn 0)))) _returnvalue_2)
    (return true)
    (else
      (return false))))

(fn Solved
  (return false))