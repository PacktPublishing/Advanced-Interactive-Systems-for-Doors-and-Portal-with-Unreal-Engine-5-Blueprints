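; Interactive door that players toggle with E inside its trigger box, with closing it setting off a celebration.
; A reversible timeline swings door and handle while a DoorState enum drives sounds and the prompt widget shown through the game mode.
; A completed close activates a tagged Niagara actor, repeats randomized firework sounds, blends to a tagged camera and disables pawn input.
; LoadDoor and GetDoorStats restore and expose door state.
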(event OnComponentBeginOverlap(Box)
  (params (OverlappedComponent :type Primitive%20Component%20Object%20Reference) (OtherActor :type Actor%20Object%20Reference) (OtherComp :type Primitive%20Component%20Object%20Reference) (OtherBodyIndex :type Integer) (bFromSweep :type Boolean) (SweepResult :type Hit%20Result%20Structure%20%28by%20ref%29))
  (if (Components|ComponentHasTag OtherComp "P")
    (Input|EnableInput (Game|GetPlayerController 0))
    (CallFunction|UpdateWidgetText)
    (Default|AddDoorWidget (Variables|Default|GetAs%20BP%20Third%20Person%20Game%20Mode) (Variables|Default|GetBox))))

(event OnComponentEndOverlap(Box)
  (params (OverlappedComponent :type Primitive%20Component%20Object%20Reference) (OtherActor :type Actor%20Object%20Reference) (OtherComp :type Primitive%20Component%20Object%20Reference) (OtherBodyIndex :type Integer))
  (if (Components|ComponentHasTag OtherComp "P")
    (Input|DisableInput (Game|GetPlayerController 0))
    (CallFunction|UpdateWidgetText)
    (Default|RemoveDoorWidget (Variables|Default|GetAs%20BP%20Third%20Person%20Game%20Mode))))

(event Custom|Do%20N%20Fireworks
  (Utilities|FlowControl|DoN 100
    (:Exit
      (Utilities|FlowControl|Delay (Math|Random|RandomFloatinRange 0.5 1.0))
      (Audio|PlaySound2D "/Game/Sounds/Fireworks_Cue.Fireworks_Cue" 1.0 (Math|Random|RandomFloatinRange 0.9 1.1) 0.0 0 0)
      (CallFunction|DoNFireworks))))

(event EventBeginPlay
  (bind _asbp_third_person_game_mode (Utilities|Casting|CastToBP_ThirdPersonGameMode (Game|GetGameMode)))
  (Variables|Default|SetAs%20BP%20Third%20Person%20Game%20Mode _asbp_third_person_game_mode)
  (Variables|Default|SetHandle%20Original%20Relative%20Rotation (Variables|/Script/Engine.SceneComponent|GetRelativeRotation (Variables|Default|Gethandle))))

(event Collision|EventActorBeginOverlap
  (params (OtherActor :type Actor%20Object%20Reference)))

(event EventTick
  (params (DeltaSeconds :type Float%20%28single-precision%29)))

(event EventLoadDoor
  (params (Door%20Stats :type ST%20Door%20Save%20Structure))
  (bind _output_get (Variables|Default|SetDoor%20State (.DoorState (Utilities|Struct|BreakST_DoorSave Door%20Stats))))
  (Transformation|SetRelativeRotation (Variables|Default|GetPropPackUE_Door1) (Math|Rotator|MakeRotator 0.0 0.0 (Utilities|Select :Index _output_get :NewEnumerator0 -9e+01 :NewEnumerator1 0.0 :NewEnumerator2 0.0 :NewEnumerator3 0.0 :NewEnumerator4 0.0)) false false))

(event Input|KeyboardEvents|E
  (params (Key :type Key%20Structure :default "None"))
  (bind _returnvalue (Game|GetPlayerController 0))
  (bind _door_sound (Variables|Default|GetDoor%20Sound))
  (bind _door_sound_2 (Variables|Default|GetDoor%20Sound))
  (:Pressed
    (Utilities|FlowControl|Sequence
      (:then_0
        (switch Utilities|FlowControl|Switch|SwitchonE_DoorState (Variables|Default|GetDoor%20State)
          (:NewEnumerator0
            (Audio|PlaySound2D "/Game/Sounds/DoorOpen_Cue.DoorOpen_Cue" 1.0 (Math|Random|RandomFloatinRange 0.8 0.99) 0.0 0 0)
            (bind (_direction _door_rotation_alpha _handle_drive) (Timeline|Timeline Reverse)
              (:Update
                (Transformation|SetRelativeRotation (Variables|Default|GetPropPackUE_Door1) (Math|Rotator|MakeRotator 0.0 0.0 (Math|Float|Lerp 0.0 9e+01 _door_rotation_alpha)) false false)
                (Transformation|SetRelativeRotation (Variables|Default|Gethandle) (Math|Rotator|Lerp(Rotator) "-90.000000,-90.000000,0.000000" "-40.000000,-90.000000,0.000000" _handle_drive true) false false)
                (Utilities|FlowControl|DoOnce false :!label _label
                  (:Completed
                    (switch Utilities|FlowControl|Switch|SwitchonETimelineDirection _direction
                      (:Forward
                        (Variables|Default|SetDoor%20State "NewEnumerator2"))
                      (:Backward
                        (Variables|Default|SetDoor%20State "NewEnumerator3"))))))
              (:Finished
                (Utilities|FlowControl|Sequence
                  (:then_0
                    (switch Utilities|FlowControl|Switch|SwitchonETimelineDirection _direction
                      (:Forward
                        (Variables|Default|SetDoor%20State "NewEnumerator0")
                        (CallFunction|UpdateWidgetText :!label _label_2)
                        (Default|AddDoorWidget (Variables|Default|GetAs%20BP%20Third%20Person%20Game%20Mode) (Variables|Default|GetBox)))
                      (:Backward
                        (Variables|Default|SetDoor%20State "NewEnumerator1")
                        (Audio|Components|Audio|Stop _door_sound_2)
                        (Audio|Components|Audio|SetSound _door_sound_2 "/Game/Sounds/DoorClose_Cue.DoorClose_Cue")
                        (Audio|Components|Audio|Play _door_sound_2 0.0)
                        (Utilities|FlowControl|Sequence
                          (:then_0
                            (goto _label_2))
                          (:then_1
                            (bind _outactors (Actor|GetAllActorswithTag "P"))
                            (bind _asniagara_actor (Utilities|Casting|CastToNiagaraActor (Utilities|Array|Get(acopy) _outactors)))
                            (Components|Activation|Activate (Variables|/Script/Niagara.NiagaraActor|GetNiagaraComponent _asniagara_actor) true)
                            (Utilities|FlowControl|DoN 100
                              (:Exit
                                (Utilities|FlowControl|Delay (Math|Random|RandomFloatinRange 0.5 1.0))
                                (Audio|PlaySound2D "/Game/Sounds/Fireworks_Cue.Fireworks_Cue" 1.0 (Math|Random|RandomFloatinRange 0.9 1.1) 0.0 0 0)
                                (CallFunction|DoNFireworks))))
                          (:then_2
                            (bind _outactors_2 (Actor|GetAllActorswithTag "C"))
                            (bind _ascamera_actor (Utilities|Casting|CastToCameraActor (Utilities|Array|Get(acopy) _outactors_2)))
                            (Game|Player|SetViewTargetwithBlend _returnvalue _ascamera_actor 2.5 "VTBlend_Linear" 0.0 false)
                            (Input|DisableInput (Pawn|GetControlledPawn _returnvalue) _returnvalue)
                            (Default|RemoveDoorWidget (Variables|Default|GetAs%20BP%20Third%20Person%20Game%20Mode)))))))
                  (:then_1
                    (goto _label Reset))))))
          (:NewEnumerator1
            (Audio|PlaySound2D "/Game/Sounds/DoorOpen_Cue.DoorOpen_Cue" 1.0 (Math|Random|RandomFloatinRange 1.0 1.15) 0.0 0 0)
            (Timeline|Timeline Play))
          (:NewEnumerator2
            (Timeline|Timeline Reverse))
          (:NewEnumerator3
            (Timeline|Timeline Play))))
      (:then_1
        (Audio|Components|Audio|Stop _door_sound)
        (Audio|Components|Audio|SetSound _door_sound "/Game/Sounds/Door_handle_Cue.Door_handle_Cue")
        (Audio|Components|Audio|Play _door_sound 0.0)))))

(fn ConstructionScript)

(fn UpdateWidgetText
  (Default|UpdateWidgetText (Variables|Default|GetAs%20BP%20Third%20Person%20Game%20Mode) (Utilities|Select :Index (Variables|Default|GetDoor%20State) :NewEnumerator0 "Close" :NewEnumerator1 "Open" :NewEnumerator2 "Close" :NewEnumerator3 "Open" :NewEnumerator4 "")))

(fn GetDoorStats
  (return (Utilities|Struct|MakeST_DoorSave (Variables|Default|GetDoor%20ID) (Variables|Default|GetDoor%20State))))

(fn Solved
  (return false))