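; Shortcut door that starts locked from the front and can only be unlocked from the back side; trying it from the front plays a rattle.
; A box overlap enables E input and shows a state-based prompt through BP_ThirdPersonGameMode.
; A player-to-door dot product decides the side and swing direction.
; A timeline swings the door open or reverses it closed, hiding the prompt while moving.
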(event OnComponentBeginOverlap(Box)
  (params (OverlappedComponent :type Primitive%20Component%20Object%20Reference) (OtherActor :type Actor%20Object%20Reference) (OtherComp :type Primitive%20Component%20Object%20Reference) (OtherBodyIndex :type Integer) (bFromSweep :type Boolean) (SweepResult :type Hit%20Result%20Structure%20%28by%20ref%29))
  (if (Components|ComponentHasTag OtherComp "P")
    (Input|EnableInput (Game|GetPlayerController 0))
    (CallFunction|UpdateWidgetText)
    (Default|AddDoorWidget (Variables|Default|GetAs%20BP%20Third%20Person%20Game%20Mode) (Variables|Default|GetBox))))

(event OnComponentEndOverlap(Box)
  (params (OverlappedComponent :type Primitive%20Component%20Object%20Reference) (OtherActor :type Actor%20Object%20Reference) (OtherComp :type Primitive%20Component%20Object%20Reference) (OtherBodyIndex :type Integer))
  (if (Components|ComponentHasTag OtherComp "P")
    (Input|DisableInput (Game|GetPlayerController 0))
    (CallFunction|UpdateWidgetText)
    (Default|RemoveDoorWidget (Variables|Default|GetAs%20BP%20Third%20Person%20Game%20Mode))))

(event Custom|Door%20Animation
  (switch Utilities|FlowControl|Switch|SwitchonE_DoorState (Variables|Default|GetDoor%20State)
    (:NewEnumerator0
      (bind (_direction _door_rotation_alpha) (Timeline|Timeline ReverseFromEnd)
        (:Update
          (Transformation|SetRelativeRotation (Variables|Default|GetPropPackUE_Door1) (Math|Rotator|MakeRotator 0.0 0.0 (Math|Float|Lerp 0.0 (Variables|Default|GetOpen%20Angle) _door_rotation_alpha)) false false)
          (Utilities|FlowControl|DoOnce false :!label _label
            (:Completed
              (switch Utilities|FlowControl|Switch|SwitchonETimelineDirection _direction
                (:Forward
                  (Variables|Default|SetDoor%20State "NewEnumerator2"))
                (:Backward
                  (Variables|Default|SetDoor%20State "NewEnumerator3")))
              (Default|RemoveDoorWidget (Variables|Default|GetAs%20BP%20Third%20Person%20Game%20Mode)))))
        (:Finished
          (Utilities|FlowControl|Sequence
            (:then_0
              (switch Utilities|FlowControl|Switch|SwitchonETimelineDirection _direction
                (:Forward
                  (Variables|Default|SetDoor%20State "NewEnumerator0"))
                (:Backward
                  (Variables|Default|SetDoor%20State "NewEnumerator1")))
              (CallFunction|UpdateWidgetText)
              (Default|AddDoorWidget (Variables|Default|GetAs%20BP%20Third%20Person%20Game%20Mode) (Variables|Default|GetBox)))
            (:then_1
              (goto _label Reset))))))
    (:NewEnumerator1
      (CallFunction|CalculateDirection)
      (Timeline|Timeline PlayFromStart))))

(event Custom|Shortcut%20Door%20Lock%20Mechanic
  (if (not (CallFunction|IsFrontside?))
    (Variables|Default|SetDoor%20State "NewEnumerator1")
    (Audio|PlaySound2D "/Game/Sounds/Door_Unlock_ue.Door_Unlock_ue" 1.0 1.0 0.0 0 0)
    (Rendering|Material|SetMaterial (Variables|Default|GetPropPackUE_Door1) 0 "/Game/Assets/Textures/Door1.Door1")
    (CallFunction|UpdateWidgetText)
    (else
      (CallFunction|DoorRattle))))

(event Custom|Door%20Rattle
  (Audio|PlaySound2D "/Game/Sounds/Door_rattle_Cue.Door_rattle_Cue" 1.0 1.0 0.0 0 0)
  (bind _door_rotation_alpha (Timeline|Timeline_0 PlayFromStart)
    (:Update
      (Transformation|SetRelativeRotation (Variables|Default|GetPropPackUE_Door1) (Math|Rotator|MakeRotator 0.0 0.0 (Math|Float|Lerp 0.0 1.5 _door_rotation_alpha)) false false))))

(event EventBeginPlay
  (bind _asbp_third_person_game_mode (Utilities|Casting|CastToBP_ThirdPersonGameMode (Game|GetGameMode)))
  (Variables|Default|SetAs%20BP%20Third%20Person%20Game%20Mode _asbp_third_person_game_mode))

(event Collision|EventActorBeginOverlap
  (params (OtherActor :type Actor%20Object%20Reference)))

(event EventTick
  (params (DeltaSeconds :type Float%20%28single-precision%29)))

(event Input|KeyboardEvents|E
  (params (Key :type Key%20Structure))
  (:Pressed
    (if (Utilities|Enum|Equal(Enum) (Variables|Default|GetDoor%20State) "NewEnumerator4")
      (CallFunction|ShortcutDoorLockMechanic)
      (else
        (CallFunction|DoorAnimation)))))

(fn ConstructionScript)

(fn UpdateWidgetText
  (Default|UpdateWidgetText (Variables|Default|GetAs%20BP%20Third%20Person%20Game%20Mode) (Utilities|Select :Index (Variables|Default|GetDoor%20State) :NewEnumerator0 "Close" :NewEnumerator1 "Open" :NewEnumerator2 "" :NewEnumerator3 "" :NewEnumerator4 (Utilities|String|SelectText "Seems Locked Form The Other Side" "Unlocked" (CallFunction|IsFrontside?)))))

(fn CalculateDirection
  (Variables|Default|SetOpen%20Angle (Math|Float|SelectFloat -9e+01 9e+01 (>= (Math|Vector|DotProduct (Math|Vector|GetUnitDirection(Vector) (Transformation|GetActorLocation) (Transformation|GetActorLocation (Game|Player|GetPlayerPawn 0))) (Transformation|GetActorForwardVector)) 0.0))))

(fn IsFrontside?
  (return (>= (Math|Vector|DotProduct (Math|Vector|GetUnitDirection(Vector) (Transformation|GetActorLocation) (Transformation|GetActorLocation (Game|Player|GetPlayerPawn 0))) (Transformation|GetActorForwardVector)) 0.0)))