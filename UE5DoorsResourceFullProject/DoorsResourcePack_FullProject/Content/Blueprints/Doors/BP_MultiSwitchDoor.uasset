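; Multi-switch door that lifts open once every linked puzzle reports solved.
; UnlockDoor checks the Puzzles array before playing a timeline that raises the door mesh, while LockDoor drives the reverse path.
; A DoorState enum tracks the motion and selects the prompt text.
; A trigger box toggles player input and the "Both Switches Need To Be On" widget through the third-person GameMode.
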(event OnComponentBeginOverlap(Box)
  (params (OverlappedComponent :type Primitive%20Component%20Object%20Reference) (OtherActor :type Actor%20Object%20Reference) (OtherComp :type Primitive%20Component%20Object%20Reference) (OtherBodyIndex :type Integer) (bFromSweep :type Boolean) (SweepResult :type Hit%20Result%20Structure%20%28by%20ref%29))
  (if (Components|ComponentHasTag OtherComp "P")
    (Input|EnableInput (Game|GetPlayerController 0))
    (CallFunction|UpdateWidgetText)
    (Default|AddDoorWidget (Variables|Default|GetAs%20BP%20Third%20Person%20Game%20Mode) (Variables|Default|GetBox))))

(event OnComponentEndOverlap(Box)
  (params (OverlappedComponent :type Primitive%20Component%20Object%20Reference) (OtherActor :type Actor%20Object%20Reference) (OtherComp :type Primitive%20Component%20Object%20Reference) (OtherBodyIndex :type Integer))
  (if (Components|ComponentHasTag OtherComp "P")
    (Input|DisableInput (Game|GetPlayerController 0))
    (CallFunction|UpdateWidgetText)
    (Default|RemoveDoorWidget (Variables|Default|GetAs%20BP%20Third%20Person%20Game%20Mode))))

(event Custom|Door%20Animation
  (bind _relative_location (Variables|Default|GetRelative%20Location))
  (bind (_x _y _z) (Math|Vector|BreakVector _relative_location))
  (switch Utilities|FlowControl|Switch|SwitchonE_DoorState (Variables|Default|GetDoor%20State)
    (:NewEnumerator0
      (if (== (Components|Timeline|GetPlaybackPosition (Variables|Default|GetAnimation%20Timeline)) 0.0)
        (bind (_direction _door_rotation_alpha) (Timeline|Animation%20Timeline Reverse)
          (:Update
            (Transformation|SetRelativeLocation (Variables|Default|GetPropPackUE_Door1) (Math|Vector|MakeVector _x _y (Math|Float|Lerp _z 2.6e+02 _door_rotation_alpha)) false false)
            (Utilities|FlowControl|DoOnce false :!label _label
              (:Completed
                (switch Utilities|FlowControl|Switch|SwitchonETimelineDirection _direction
                  (:Forward
                    (Variables|Default|SetDoor%20State "NewEnumerator2"))
                  (:Backward
                    (Variables|Default|SetDoor%20State "NewEnumerator3")))
                (Default|RemoveDoorWidget (Variables|Default|GetAs%20BP%20Third%20Person%20Game%20Mode)))))
          (:Finished
            (Utilities|FlowControl|Sequence
              (:then_0
                (switch Utilities|FlowControl|Switch|SwitchonETimelineDirection _direction
                  (:Forward
                    (Variables|Default|SetDoor%20State "NewEnumerator0"))
                  (:Backward
                    (Variables|Default|SetDoor%20State "NewEnumerator1")
                    (Default|AddDoorWidget (Variables|Default|GetAs%20BP%20Third%20Person%20Game%20Mode) (Variables|Default|GetBox))))
                (CallFunction|UpdateWidgetText))
              (:then_1
                (goto _label Reset)))))
        (else
          (Audio|PlaySound2D "/Game/Sounds/DoorLift_Cue.DoorLift_Cue" 1.0 0.8 0.0 0 0)
          (Timeline|Animation%20Timeline Reverse))))
    (:NewEnumerator1
      (Audio|PlaySound2D "/Game/Sounds/DoorLift_Cue.DoorLift_Cue" 1.0 1.0 0.0 0 0)
      (Timeline|Animation%20Timeline Play))))

(event EventBeginPlay
  (bind _asbp_third_person_game_mode (Utilities|Casting|CastToBP_ThirdPersonGameMode (Game|GetGameMode)))
  (Variables|Default|SetAs%20BP%20Third%20Person%20Game%20Mode _asbp_third_person_game_mode)
  (Variables|Default|SetRelative%20Location (Variables|/Script/Engine.SceneComponent|GetRelativeLocation (Variables|Default|GetPropPackUE_Door1))))

(event Collision|EventActorBeginOverlap
  (params (OtherActor :type Actor%20Object%20Reference)))

(event EventTick
  (params (DeltaSeconds :type Float%20%28single-precision%29)))

(event EventUnlockDoor
  (bind _all_puzzles_solved (CallFunction|CheckPuzzleAnswers))
  (if _all_puzzles_solved
    (Variables|Default|SetDoor%20State "NewEnumerator1")
    (Default|RemoveDoorWidget (Variables|Default|GetAs%20BP%20Third%20Person%20Game%20Mode))
    (CallFunction|DoorAnimation)))

(event EventLockDoor
  (Variables|Default|SetDoor%20State "NewEnumerator0")
  (CallFunction|DoorAnimation))

(fn ConstructionScript)

(fn UpdateWidgetText
  (Default|UpdateWidgetText (Variables|Default|GetAs%20BP%20Third%20Person%20Game%20Mode) (Utilities|Select :Index (Variables|Default|GetDoor%20State) :NewEnumerator0 "" :NewEnumerator1 "Both Switches Need To Be On" :NewEnumerator2 "" :NewEnumerator3 "" :NewEnumerator4 "")))

(fn CheckPuzzleAnswers
  (bind _array_element (Utilities|Array|ForEachLoopwithBreak (Variables|Default|GetPuzzles) :!label _label)
    (:LoopBody
      (bind _solved (Class|BIDoors|Solved(Message) _array_element))
      (if (not _solved)
        (LocalVariables|SetAll%20Solved false)
        (goto _label Break)))
    (:Completed
      (return (LocalVariables|GetAll%20Solved)))))

(fn Solved
  (return false))