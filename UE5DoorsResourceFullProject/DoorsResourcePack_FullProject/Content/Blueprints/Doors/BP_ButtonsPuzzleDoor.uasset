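; Sliding puzzle door that opens on UnlockDoor and closes on LockDoor, each with a slide sound.
; A single timeline moves the door mesh along relative Y by OpenDisplacement, playing forward to open and reversing to close unless already at the start.
; Timeline direction sets DoorState, with a DoOnce marking the moving state until Finished sets the end state and resets it.
; The Solved function is a stub returning false, and nothing here calls it.
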(event EventBeginPlay)

(event Collision|EventActorBeginOverlap
  (params (OtherActor :type Actor%20Object%20Reference)))

(event EventTick
  (params (DeltaSeconds :type Float%20%28single-precision%29)))

(event EventUnlockDoor
  (Audio|PlaySound2D "/Game/Sounds/SlideDoor_Cue.SlideDoor_Cue" 1.0 0.8 0.0 0 0)
  (bind (_direction _door_rotation_alpha) (Timeline|Animation%20Timeline Play)
    (:Update
      (Transformation|SetRelativeLocation (Variables|Default|GetPropPackUE_Door1) (Math|Vector|MakeVector 0.0 (Math|Float|Lerp 0.0 (Variables|Default|GetOpen%20Displacement) _door_rotation_alpha) 0.0) false false)
      (Utilities|FlowControl|DoOnce false :!label _label
        (:Completed
          (switch Utilities|FlowControl|Switch|SwitchonETimelineDirection _direction
            (:Forward
              (Variables|Default|SetDoor%20State "NewEnumerator2"))
            (:Backward
              (Variables|Default|SetDoor%20State "NewEnumerator3"))))))
    (:Finished
      (Utilities|FlowControl|Sequence
        (:then_0
          (switch Utilities|FlowControl|Switch|SwitchonETimelineDirection _direction
            (:Forward
              (Variables|Default|SetDoor%20State "NewEnumerator0"))
            (:Backward
              (Variables|Default|SetDoor%20State "NewEnumerator1"))))
        (:then_1
          (goto _label Reset))))))

(event EventLockDoor
  (if (not (== (Components|Timeline|GetPlaybackPosition (Variables|Default|GetAnimation%20Timeline)) 0.0))
    (Audio|PlaySound2D "/Game/Sounds/SlideDoor_Cue.SlideDoor_Cue" 1.0 0.7 0.0 0 0)
    (bind (_direction _door_rotation_alpha) (Timeline|Animation%20Timeline Reverse)
      (:Update
        (Transformation|SetRelativeLocation (Variables|Default|GetPropPackUE_Door1) (Math|Vector|MakeVector 0.0 (Math|Float|Lerp 0.0 (Variables|Default|GetOpen%20Displacement) _door_rotation_alpha) 0.0) false false)
        (Utilities|FlowControl|DoOnce false :!label _label
          (:Completed
            (switch Utilities|FlowControl|Switch|SwitchonETimelineDirection _direction
              (:Forward
                (Variables|Default|SetDoor%20State "NewEnumerator2"))
              (:Backward
                (Variables|Default|SetDoor%20State "NewEnumerator3"))))))
      (:Finished
        (Utilities|FlowControl|Sequence
          (:then_0
            (switch Utilities|FlowControl|Switch|SwitchonETimelineDirection _direction
              (:Forward
                (Variables|Default|SetDoor%20State "NewEnumerator0"))
              (:Backward
                (Variables|Default|SetDoor%20State "NewEnumerator1"))))
          (:then_1
            (goto _label Reset)))))))

(fn ConstructionScript)

(fn Solved
  (return false))