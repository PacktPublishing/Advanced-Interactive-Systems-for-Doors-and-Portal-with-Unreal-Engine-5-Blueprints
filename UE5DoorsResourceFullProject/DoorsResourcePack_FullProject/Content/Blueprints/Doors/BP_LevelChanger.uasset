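; BP_LevelChanger is a trigger actor that moves the player to another level when the third-person character enters its box.
; The overlap shows a fade widget and plays a teleport sound that persists across the level transition.
; After the fade animation's length plus a short pause, it flags the game instance as loaded, saves door state and calls LevelTransfer with its ComeFrom value.
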(event OnComponentBeginOverlap(Box)
  (params (OverlappedComponent :type Primitive%20Component%20Object%20Reference) (OtherActor :type Actor%20Object%20Reference) (OtherComp :type Primitive%20Component%20Object%20Reference) (OtherBodyIndex :type Integer) (bFromSweep :type Boolean) (SweepResult :type Hit%20Result%20Structure%20%28by%20ref%29))
  (bind _returnvalue (Game|GetGameInstance))
  (bind _asgi_doors_tutorial (Utilities|Casting|CastToGI_DoorsTutorial _returnvalue))
  (Utilities|Casting|CastToBP_ThirdPersonCharacter OtherActor)
  (bind _returnvalue_2 (UserInterface|CreateWidget "/Game/UI/WG_Fade.WG_Fade_C" (Game|GetPlayerController 0)))
  (UserInterface|Viewport|AddtoViewport _returnvalue_2 0)
  (UserInterface|Animation|PlayAnimation _returnvalue_2 (Variables|/Game/UI/WG_Fade.WG_Fade_C|GetMy_Fade_Animation _returnvalue_2) 0.0 1 "Forward" 1.0 false)
  (bind _returnvalue_3 (Audio|SpawnSound2D "/Engine/VREditor/Sounds/VR_teleport_Cue.VR_teleport_Cue" 1.0 1.0 0.0 0 true))
  (Audio|Components|Audio|Play _returnvalue_3 0.0)
  (Utilities|FlowControl|Delay (+ (Class|WidgetAnimation|GetEndTime (Variables|/Game/UI/WG_Fade.WG_Fade_C|GetMy_Fade_Animation _returnvalue_2)) 0.5))
  (Variables|/Game/Blueprints/GI_DoorsTutorial.GI_DoorsTutorial_C|SetLoaded%20Game _asgi_doors_tutorial true)
  (Default|SaveDoors _asgi_doors_tutorial)
  (Default|LevelTransfer _asgi_doors_tutorial (Variables|Default|GetCome%20From)))

(event EventBeginPlay)

(event Collision|EventActorBeginOverlap
  (params (OtherActor :type Actor%20Object%20Reference)))

(event EventTick
  (params (DeltaSeconds :type Float%20%28single-precision%29)))

(fn ConstructionScript)