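; BP_Switch is a pressure plate that unlocks a linked door while something rests on it.
; Box overlaps play a timeline that lerps the plate mesh down; on forward completion it sets IsSolved, swaps to the lit material and sends the door an unlock message.
; When the box empties, it immediately clears IsSolved, restores the material, relocks the door and reverses the timeline.
; The Solved function exposes the current state.
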(event OnComponentBeginOverlap(Box)
  (params (OverlappedComponent :type Primitive%20Component%20Object%20Reference) (OtherActor :type Actor%20Object%20Reference) (OtherComp :type Primitive%20Component%20Object%20Reference) (OtherBodyIndex :type Integer) (bFromSweep :type Boolean) (SweepResult :type Hit%20Result%20Structure%20%28by%20ref%29))
  (if (not (<= (Utilities|Array|Length (Collision|GetOverlappingActors (Variables|Default|GetBox) 0 :!class /Script/Engine.PrimitiveComponent)) 0))
    (bind (_direction _newtrack_0) (Timeline|Timeline Play)
      (:Update
        (Transformation|SetRelativeLocation (Variables|Default|GetStaticMesh1) (Math|Vector|MakeVector 0.0 0.0 (Math|Float|Lerp 0.0 -1e+01 _newtrack_0)) false false))
      (:Finished
        (switch Utilities|FlowControl|Switch|SwitchonETimelineDirection _direction
          (:Forward
            (Variables|Default|SetIsSolved true)
            (Rendering|Material|SetMaterial (Variables|Default|GetStaticMesh1) 0 "/Game/Assets/Textures/PressurePlateOn.PressurePlateOn")
            (Class|BIDoors|UnlockDoor(Message) (Variables|Default|GetDoor))))))))

(event OnComponentEndOverlap(Box)
  (params (OverlappedComponent :type Primitive%20Component%20Object%20Reference) (OtherActor :type Actor%20Object%20Reference) (OtherComp :type Primitive%20Component%20Object%20Reference) (OtherBodyIndex :type Integer))
  (if (<= (Utilities|Array|Length (Collision|GetOverlappingActors (Variables|Default|GetBox) 0 :!class /Script/Engine.PrimitiveComponent)) 0)
    (Variables|Default|SetIsSolved false)
    (Rendering|Material|SetMaterial (Variables|Default|GetStaticMesh1) 0 "/Game/Assets/Textures/PressurePlate.PressurePlate")
    (Class|BIDoors|LockDoor(Message) (Variables|Default|GetDoor))
    (bind (_direction _newtrack_0) (Timeline|Timeline Reverse)
      (:Update
        (Transformation|SetRelativeLocation (Variables|Default|GetStaticMesh1) (Math|Vector|MakeVector 0.0 0.0 (Math|Float|Lerp 0.0 -1e+01 _newtrack_0)) false false))
      (:Finished
        (switch Utilities|FlowControl|Switch|SwitchonETimelineDirection _direction
          (:Forward
            (Variables|Default|SetIsSolved true)
            (Rendering|Material|SetMaterial (Variables|Default|GetStaticMesh1) 0 "/Game/Assets/Textures/PressurePlateOn.PressurePlateOn")
            (Class|BIDoors|UnlockDoor(Message) (Variables|Default|GetDoor))))))))

(event EventBeginPlay)

(event Collision|EventActorBeginOverlap
  (params (OtherActor :type Actor%20Object%20Reference)))

(event EventTick
  (params (DeltaSeconds :type Float%20%28single-precision%29)))

(fn ConstructionScript)

(fn Solved
  (return (Variables|Default|GetIsSolved)))